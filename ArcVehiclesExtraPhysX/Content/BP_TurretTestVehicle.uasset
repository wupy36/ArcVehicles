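; BP_TurretTestVehicle is a drivable four-wheeled vehicle Blueprint, named as a test vehicle for turrets, though this file contains no turret logic.
; MoveForward and MoveRight axes feed throttle and steering on the WheeledVehicleMovementComponent4W, and holding Jump applies the handbrake.
; A hardcoded E key calls RequestLeaveVehicle with the PlayerState to request an exit, and BeginPlay only calls the parent.
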(event EventBeginPlay
  (|CallParentFunction))

(event Collision|EventActorBeginOverlap
  (params (OtherActor :type Actor%20Object%20Reference)))

(event EventTick
  (params (DeltaSeconds :type Float%20%28single-precision%29)))

(event Input|ActionEvents|InputActionJump
  (params (Key :type Key%20Structure :default "None"))
  (bind _wheeledvehiclemovementcomponent4w (Variables|Default|GetWheeledVehicleMovementComponent4W))
  (:Pressed
    (Class|WheeledVehicleMovementComponent|SetHandbrakeInput _wheeledvehiclemovementcomponent4w true))
  (:Released
    (Class|WheeledVehicleMovementComponent|SetHandbrakeInput _wheeledvehiclemovementcomponent4w false)))

(event Input|AxisEvents|InputAxisMoveForward
  (params (AxisValue :type Float%20%28single-precision%29))
  (Class|WheeledVehicleMovementComponent|SetThrottleInput (Variables|Default|GetWheeledVehicleMovementComponent4W) AxisValue))

(event Input|AxisEvents|InputAxisMoveRight
  (params (AxisValue :type Float%20%28single-precision%29))
  (Class|WheeledVehicleMovementComponent|SetSteeringInput (Variables|Default|GetWheeledVehicleMovementComponent4W) AxisValue))

(event Input|KeyboardEvents|E
  (params (Key :type Key%20Structure :default "None"))
  (:Pressed
    (Class|ArcBaseVehicle|RequestLeaveVehicle (Variables|Default|GetPlayerState))))

(fn ConstructionScript)