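; Sample player controller that lets the player enter and exit Arc vehicles with the E key.
; A sample character with a valid seat config exits that seat's vehicle; otherwise a short debug-drawn trace along the camera's forward vector finds a vehicle and requests any seat.
; Entry calls the vehicle directly on authority or through TryGetInVehicle on remote.
; When the controlled pawn is itself an Arc vehicle, E requests leaving it.
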(event Custom|TryGetInVehicle
  (params (Vehicle :type Arc%20Base%20Vehicle%20Object%20Reference))
  (Class|ArcBaseVehicle|RequestEnterAnySeat Vehicle (Variables|GetPlayerState)))

(event Custom|RequestExitVehicle
  (params (Vehicle :type Arc%20Base%20Vehicle%20Object%20Reference))
  (Class|ArcBaseVehicle|RequestLeaveVehicle Vehicle (Variables|GetPlayerState)))

(event EventBeginPlay)

(event EventTick
  (params (DeltaSeconds :type Float%20%28single-precision%29)))

(event Input|KeyboardEvents|E
  (params (Key :type Key%20Structure :default "None"))
  (bind _returnvalue (Pawn|GetControlledPawn))
  (:Pressed
    (bind _asbp_vehicle_sample_character (Utilities|Casting|CastToBP_VehicleSampleCharacter _returnvalue)
      (:then
        (Utilities|IsValid (Actor|GetComponentbyClass _asbp_vehicle_sample_character "/Script/ArcVehicles.ArcVehiclePlayerSeatComponent")
          (:Is%20Valid
            (Utilities|IsValid (Variables|/Script/ArcVehicles.ArcVehiclePlayerSeatComponent|GetSeatConfig (Actor|GetComponentbyClass _asbp_vehicle_sample_character "/Script/ArcVehicles.ArcVehiclePlayerSeatComponent"))
              (:Is%20Valid
                (CallFunction|RequestExitVehicle (Class|ArcVehicleSeatConfig|GetVehicleOwner (Variables|/Script/ArcVehicles.ArcVehiclePlayerSeatComponent|GetSeatConfig (Actor|GetComponentbyClass _asbp_vehicle_sample_character "/Script/ArcVehicles.ArcVehiclePlayerSeatComponent")))))
              (:Is%20Not%20Valid
                (bind (_outhit _returnvalue_2) (Collision|LineTraceForObjects (Transformation|GetActorLocation _asbp_vehicle_sample_character) (+ (Transformation|GetActorLocation _asbp_vehicle_sample_character) (* (Math|Vector|GetForwardVector (Variables|/ArcVehiclesExtra/BP_VehicleSampleCharacter.BP_VehicleSampleCharacter_C|GetFirstPersonCamera _asbp_vehicle_sample_character)) 5e+02)) (Utilities|Array|MakeArray "ObjectTypeQuery5") false 0 "ForDuration" :!label _label))
                (if _returnvalue_2
                  (bind _asarc_base_vehicle (Utilities|Casting|CastToArcBaseVehicle (.HitActor (Collision|BreakHitResult _outhit))))
                  (Networking|SwitchHasAuthority
                    (:Authority
                      (Class|ArcBaseVehicle|RequestEnterAnySeat _asarc_base_vehicle (Variables|GetPlayerState)))
                    (:Remote
                      (CallFunction|TryGetinVehicle _asarc_base_vehicle)))))))
          (:Is%20Not%20Valid
            (goto _label))))
      (:CastFailed
        (bind _asarc_base_vehicle_2 (Utilities|Casting|CastToArcBaseVehicle _returnvalue))
        (CallFunction|RequestExitVehicle _asarc_base_vehicle_2)))))

(fn ConstructionScript)